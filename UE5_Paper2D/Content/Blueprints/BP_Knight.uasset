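; BP_Knight is a 2D knight that changes its facing flipbook in response to player input.
; The MoveUp and MoveRight axis events pick an up, down or side idle flipbook by the sign of non-zero input.
; Left and right share the side flipbook, with the sprite rotated 180 degrees for left.
; Each direction prints a debug label, and the graph applies no movement.
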(event `InputAxis|MoveUp`
  (params (AxisValue :type "Float (single-precision)"))
  (bind _sprite (`self.Sprite`))
  (if (== AxisValue 0.0)
    _
    (elif (> AxisValue 0.0)
      (`PaperFlipbookComponent.SetFlipbook` _sprite "/Game/Knight/up_idle.up_idle")
      (`KismetSystemLibrary.PrintText` "up")
      (else
        (`PaperFlipbookComponent.SetFlipbook` _sprite "/Game/Knight/down_idle.down_idle")
        (`KismetSystemLibrary.PrintText` "down")))))

(event `InputAxis|MoveRight`
  (params (AxisValue :type "Float (single-precision)"))
  (bind _sprite (`self.Sprite`))
  (if (== AxisValue 0.0)
    _
    (elif (> AxisValue 0.0)
      (`PaperFlipbookComponent.SetFlipbook` _sprite "/Game/Knight/side_idle.side_idle")
      (`SceneComponent.K2_SetRelativeRotation` _sprite (struct) false false)
      (`KismetSystemLibrary.PrintText` "right")
      (else
        (`PaperFlipbookComponent.SetFlipbook` _sprite "/Game/Knight/side_idle.side_idle")
        (`SceneComponent.K2_SetRelativeRotation` _sprite (struct :`Yaw` 180.0) false false)
        (`KismetSystemLibrary.PrintText` "left")))))

(fn `UserConstructionScript`)